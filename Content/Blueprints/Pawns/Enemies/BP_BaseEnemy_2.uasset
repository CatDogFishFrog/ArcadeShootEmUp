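; BP_BaseEnemy_2 is an enemy that continuously homes in on the player pawn.
; It caches player 0's pawn on BeginPlay and acts each Tick only while that pawn casts to BP_PlayerPawn.
; It moves forward by a fixed, unswept local step per frame, independent of delta time.
; Steering is yaw-only: the look-at difference is clamped to ±RotationSpeed, then scaled by delta time.
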(event EventTick
  (params (DeltaSeconds :type Float%20%28single-precision%29))
  (bind _rotationspeed (Variables|Default|GetRotationSpeed))
  (|CallParentFunction DeltaSeconds)
  (Utilities|Casting|CastToBP_PlayerPawn (Variables|Default|GetPlayerPawn))
  (if (stale _bsuccess)
    (Transformation|AddActorLocalOffset "5.000000, 0, 0" false false)
    (Transformation|AddActorLocalRotation (Math|Rotator|MakeRotator 0.0 0.0 (* (Math|Float|Clamp(Float) (.yaw (Math|Rotator|Delta(Rotator) (Math|Rotator|FindLookatRotation (Transformation|GetActorLocation) (Transformation|GetActorLocation (Variables|Default|GetPlayerPawn))) (Transformation|GetActorRotation))) (* _rotationspeed -1.0) _rotationspeed) (Utilities|Time|GetWorldDeltaSeconds))) false false)))

(event EventBeginPlay
  (|CallParentFunction)
  (Variables|Default|SetPlayerPawn (Game|Player|GetPlayerPawn 0)))

(fn ConstructionScript)