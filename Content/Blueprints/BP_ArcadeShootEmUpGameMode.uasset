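; BP_ArcadeShootEmUpGameMode is the shoot 'em up game mode that handles main menu startup and best-score checks.
; BeginPlay creates a fresh MySave as SaveVar, then reads slot "1" and, if OpenMM is set, shows W_MainMenu and pauses.
; CheckBestScore compares GamePoints with slot "2" BestPoints and calls SaveBestScore on SaveVar when higher.
; Both checks do nothing if loading or casting the save fails.
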(event `self.ReceiveBeginPlay`
  (bind _returnvalue (`GameplayStatics.CreateSaveGameObject` "/Game/Blueprints/SaveGame/MySave.MySave_C"))
  (set `self.SaveVar` _returnvalue)
  (bind _returnvalue_2 (`GameplayStatics.LoadGameFromSlot` "1"))
  (bind _asmy_save (cast `/Game/Blueprints/SaveGame/MySave` _returnvalue_2))
  (if (`/Game/Blueprints/SaveGame/MySave.OpenMM` _asmy_save)
    (bind _returnvalue_3 (`|CreateWidget` "/Game/UI/MainMenu/W_MainMenu.W_MainMenu_C"))
    (`UserWidget.AddToViewport` _returnvalue_3 0)
    (`GameplayStatics.SetGamePaused` true)))

(fn `CheckBestScore`
  (bind _returnvalue (`GameplayStatics.LoadGameFromSlot` "2"))
  (bind _asmy_save (cast `/Game/Blueprints/SaveGame/MySave` _returnvalue))
  (if (< (`/Game/Blueprints/SaveGame/MySave.BestPoints` _asmy_save) (`self.GamePoints`))
    (`/Game/Blueprints/SaveGame/MySave.SaveBestScore` (`self.SaveVar`) (`self.GamePoints`))))

(fn `GetSaveVar`
  (returns (SaveVar :type "SaveGame Object Reference"))
  (return (`self.SaveVar`)))

(fn `UserConstructionScript`)